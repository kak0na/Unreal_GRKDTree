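; KD-tree demo actor that visualizes spatial queries around the player pawn.
; BeginPlay scatters random points on a flat square, builds the tree from them, spawns a BP_Cube at each and runs an in-order traversal.
; Each Tick, QueryType selects nearest, N-nearest, radius or N-nearest-in-frustum search; all cube materials reset, then the returned indices are highlighted.
; The tree functions are called here but defined outside this graph.
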(event `self.ReceiveBeginPlay`
  (`|ExecutionSequence`
    (:`then_0`
      (`KismetArrayLibrary.Array_Clear` (`self.Points_0`))
      (for _ (range 100)
        (`KismetArrayLibrary.Array_Add` (`self.Points_0`) (`KismetMathLibrary.RandomPointInBoundingBox_Box` (`KismetMathLibrary.MakeBox` (0.0 0.0 0.0) (1000.0 1000.0 0.0))))))
    (:`then_1`
      (`self.BuildKDtree` (`self.Points_0`))
      (`KismetArrayLibrary.Array_Clear` (`self.BP_Spheres`))
      (for _array_element (`self.Points_0`)
        (bind _returnvalue (`|SpawnActorFromClass` "/Game/GRKDTreeDemo/BP_Cube.BP_Cube_C" (`KismetMathLibrary.Conv_VectorToTransform` _array_element) "Undefined" "OverrideRootScale" null null))
        (`KismetArrayLibrary.Array_Add` (`self.BP_Spheres`) _returnvalue)))
    (:`then_2`
      (`self.InOrderTraversal`))))

(event `self.ReceiveTick`
  (params (DeltaSeconds :type "Float (single-precision)"))
  (`parent.ReceiveTick` DeltaSeconds)
  (switch `int` (`self.QueryType`)
    (:`0`
      (bind _index (`self.FindNearestNeighbor` (`self.K2_GetActorLocation` (`GameplayStatics.GetPlayerPawn` 0))))
      (`/Game/GRKDTreeDemo/BP_Cube.SetMaterial` (`self.BP_Spheres`) false)
      (`/Game/GRKDTreeDemo/BP_Cube.SetMaterial` (`|GetArrayItem` (`self.BP_Spheres`) _index) true))
    (:`1`
      (bind _outindices (`self.FindNearestNNeighbors` (`self.K2_GetActorLocation` (`GameplayStatics.GetPlayerPawn` 0)) 10))
      (`/Game/GRKDTreeDemo/BP_Cube.SetMaterial` (`self.BP_Spheres`) false)
      (for _array_element _outindices
        (`/Game/GRKDTreeDemo/BP_Cube.SetMaterial` (`|GetArrayItem` (`self.BP_Spheres`) _array_element) true)))
    (:`2`
      (bind _outindices_2 (`self.FindSphereWithIndexs` (`self.K2_GetActorLocation` (`GameplayStatics.GetPlayerPawn` 0)) 300.0))
      (`/Game/GRKDTreeDemo/BP_Cube.SetMaterial` (`self.BP_Spheres`) false)
      (for _array_element_2 _outindices_2
        (`/Game/GRKDTreeDemo/BP_Cube.SetMaterial` (`|GetArrayItem` (`self.BP_Spheres`) _array_element_2) true)))
    (:`3`
      (bind _outindices_3 (`self.FindNearestNInFrustum` (`self.K2_GetActorLocation` (`GameplayStatics.GetPlayerPawn` 0)) 10))
      (`/Game/GRKDTreeDemo/BP_Cube.SetMaterial` (`self.BP_Spheres`) false)
      (for _array_element_3 _outindices_3
        (`/Game/GRKDTreeDemo/BP_Cube.SetMaterial` (`|GetArrayItem` (`self.BP_Spheres`) _array_element_3) true)))))

(fn `UserConstructionScript`)